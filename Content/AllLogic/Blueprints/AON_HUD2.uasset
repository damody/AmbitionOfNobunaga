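; HUD Blueprint that hosts the hero UI and draws a custom cursor material at the mouse position, plus text readouts of the current and initial mouse coordinates.
; BeginPlay creates the HeroUse widget and adds it to the viewport, and hero select and unselect events set or clear its hero.
; GetEquipmentPosition and GetSkillPosition map an index to that widget's canvas slot position and size, returning zero on failure.
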(event `self.ReceiveDrawHUD`
  (params (SizeX :type Integer) (SizeY :type Integer))
  (bind (_currentmousexy_x _currentmousexy_y) (`KismetMathLibrary.BreakVector2D` (`self.CurrentMouseXY`)))
  (bind (_initialmousexy_x _initialmousexy_y) (`KismetMathLibrary.BreakVector2D` (`self.InitialMouseXY`)))
  (bind (_locationx _locationy) (`PlayerController.GetMousePosition` (`GameplayStatics.GetPlayerController` 0)))
  (`self.DrawText` (`KismetStringLibrary.Concat_StrStr` (`KismetStringLibrary.Concat_StrStr` (`KismetStringLibrary.Conv_DoubleToString` _currentmousexy_x) ",") (`KismetStringLibrary.Conv_DoubleToString` _currentmousexy_y)) (struct :`R` 1.0 :`G` 1.0 :`B` 1.0 :`A` 1.0) 256.0 0.0 "/Engine/EngineFonts/Roboto.Roboto")
  (`self.DrawText` (`KismetStringLibrary.Concat_StrStr` (`KismetStringLibrary.Concat_StrStr` (`KismetStringLibrary.Conv_DoubleToString` _initialmousexy_x) ",") (`KismetStringLibrary.Conv_DoubleToString` _initialmousexy_y)) (struct :`R` 1.0 :`G` 1.0 :`B` 1.0 :`A` 1.0) 256.0 30.0 "/Engine/EngineFonts/Roboto.Roboto")
  (`self.DrawMaterialSimple` "/Game/AllLogic/mouse/M_gam1541.M_gam1541" _locationx _locationy 25.0 25.0))

(event `self.ReceiveBeginPlay`
  (bind _returnvalue (`|CreateWidget` "/Game/AllLogic/UI/HeroUse.HeroUse_C"))
  (bind _output_get (set `self.HeroUI` _returnvalue))
  (`UserWidget.AddToViewport` _returnvalue 0)
  (`UserWidget.AddToViewport` _output_get 0))

(event `self.SelectedHero`
  (params (hero :type "HeroCharacter Object Reference"))
  (`/Game/AllLogic/UI/HeroUse.SetHero` (`self.HeroUI`) hero))

(event `self.UnSelectHero`
  (`/Game/AllLogic/UI/HeroUse.ClearHero` (`self.HeroUI`)))

(fn `GetEquipmentPosition`
  (params (n :type Integer))
  (returns (pos :type "Vector2D Structure") (size :type "Vector2D Structure"))
  (switch `int` n
    (:`Default`
      _)
    (:`0`
      (bind _ascanvas_panel_slot (cast `CanvasPanelSlot` (`Widget.Slot` (`/Game/AllLogic/UI/HeroUse.RefEquipment1` (`self.HeroUI`))))
        (:`then`
          (return (`CanvasPanelSlot.GetPosition` _ascanvas_panel_slot) (`CanvasPanelSlot.GetSize` _ascanvas_panel_slot)))
        (:`CastFailed`
          _)))
    (:`1`
      (bind _ascanvas_panel_slot_2 (cast `CanvasPanelSlot` (`Widget.Slot` (`/Game/AllLogic/UI/HeroUse.RefEquipment2` (`self.HeroUI`))))
        (:`then`
          (return (`CanvasPanelSlot.GetPosition` _ascanvas_panel_slot_2) (`CanvasPanelSlot.GetSize` _ascanvas_panel_slot_2)))
        (:`CastFailed`
          _)))
    (:`2`
      (bind _ascanvas_panel_slot_3 (cast `CanvasPanelSlot` (`Widget.Slot` (`/Game/AllLogic/UI/HeroUse.RefEquipment3` (`self.HeroUI`))))
        (:`then`
          (return (`CanvasPanelSlot.GetPosition` _ascanvas_panel_slot_3) (`CanvasPanelSlot.GetSize` _ascanvas_panel_slot_3)))
        (:`CastFailed`
          _)))
    (:`3`
      (bind _ascanvas_panel_slot_4 (cast `CanvasPanelSlot` (`Widget.Slot` (`/Game/AllLogic/UI/HeroUse.RefEquipment4` (`self.HeroUI`))))
        (:`then`
          (return (`CanvasPanelSlot.GetPosition` _ascanvas_panel_slot_4) (`CanvasPanelSlot.GetSize` _ascanvas_panel_slot_4)))
        (:`CastFailed`
          _)))
    (:`4`
      (bind _ascanvas_panel_slot_5 (cast `CanvasPanelSlot` (`Widget.Slot` (`/Game/AllLogic/UI/HeroUse.RefEquipment5` (`self.HeroUI`))))
        (:`then`
          (return (`CanvasPanelSlot.GetPosition` _ascanvas_panel_slot_5) (`CanvasPanelSlot.GetSize` _ascanvas_panel_slot_5)))
        (:`CastFailed`
          _)))
    (:`5`
      (bind _ascanvas_panel_slot_6 (cast `CanvasPanelSlot` (`Widget.Slot` (`/Game/AllLogic/UI/HeroUse.RefEquipment6` (`self.HeroUI`))))
        (:`then`
          (return (`CanvasPanelSlot.GetPosition` _ascanvas_panel_slot_6) (`CanvasPanelSlot.GetSize` _ascanvas_panel_slot_6)))
        (:`CastFailed`
          _))))
  (return (0.0 0.0) (0.0 0.0)))

(fn `GetSkillPosition`
  (params (n :type Integer))
  (returns (pos :type "Vector2D Structure") (size :type "Vector2D Structure"))
  (switch `int` n
    (:`Default`
      _)
    (:`0`
      (bind _ascanvas_panel_slot (cast `CanvasPanelSlot` (`Widget.Slot` (`/Game/AllLogic/UI/HeroUse.Btn_Skill1` (`self.HeroUI`))))
        (:`then`
          (return (`CanvasPanelSlot.GetPosition` _ascanvas_panel_slot) (`CanvasPanelSlot.GetSize` _ascanvas_panel_slot)))
        (:`CastFailed`
          _)))
    (:`1`
      (bind _ascanvas_panel_slot_2 (cast `CanvasPanelSlot` (`Widget.Slot` (`/Game/AllLogic/UI/HeroUse.Btn_Skill2` (`self.HeroUI`))))
        (:`then`
          (return (`CanvasPanelSlot.GetPosition` _ascanvas_panel_slot_2) (`CanvasPanelSlot.GetSize` _ascanvas_panel_slot_2)))
        (:`CastFailed`
          _)))
    (:`2`
      (bind _ascanvas_panel_slot_3 (cast `CanvasPanelSlot` (`Widget.Slot` (`/Game/AllLogic/UI/HeroUse.Btn_Skill3` (`self.HeroUI`))))
        (:`then`
          (return (`CanvasPanelSlot.GetPosition` _ascanvas_panel_slot_3) (`CanvasPanelSlot.GetSize` _ascanvas_panel_slot_3)))
        (:`CastFailed`
          _)))
    (:`3`
      (bind _ascanvas_panel_slot_4 (cast `CanvasPanelSlot` (`Widget.Slot` (`/Game/AllLogic/UI/HeroUse.Btn_Skill4` (`self.HeroUI`))))
        (:`then`
          (return (`CanvasPanelSlot.GetPosition` _ascanvas_panel_slot_4) (`CanvasPanelSlot.GetSize` _ascanvas_panel_slot_4)))
        (:`CastFailed`
          _))))
  (return (0.0 0.0) (0.0 0.0)))

(fn `UserConstructionScript`)