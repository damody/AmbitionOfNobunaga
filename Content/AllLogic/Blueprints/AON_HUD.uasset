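; AON_HUD is a HUD that shows the hero's four-skill interface and tracks each skill's cooldown.
; On BeginPlay it creates the HeroUse widget with all skills ready, then Tick advances per-skill timers and sends progress ratios to the widget.
; Each skill event triggers the widget and resets its timer only if the cooldown has elapsed.
; DrawHUD prints mouse coordinates and draws a material at the cursor position.
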(event `self.ReceiveBeginPlay`
  (bind _returnvalue (`|CreateWidget` "/Game/AllLogic/UI/HeroUse.HeroUse_C"))
  (bind _output_get (set `self.HeroUI` _returnvalue))
  (`UserWidget.AddToViewport` _returnvalue 0)
  (`UserWidget.AddToViewport` _output_get 0)
  (set `self.Skill1_CD_real` (`self.Skill1_CD`))
  (set `self.Skill2_CD_real` (`self.Skill2_CD`))
  (set `self.Skill3_CD_real` (`self.Skill3_CD`))
  (set `self.Skill4_CD_real` (`self.Skill4_CD`)))

(event `self.ReceiveTick`
  (params (DeltaSeconds :type "Float (single-precision)"))
  (set `self.Skill1_CD_real` (+ DeltaSeconds (`self.Skill1_CD_real`)))
  (set `self.Skill2_CD_real` (+ DeltaSeconds (`self.Skill2_CD_real`)))
  (set `self.Skill3_CD_real` (+ DeltaSeconds (`self.Skill3_CD_real`)))
  (set `self.Skill4_CD_real` (+ DeltaSeconds (`self.Skill4_CD_real`)))
  (`/Game/AllLogic/UI/HeroUse.SetSkill1 Progress` (`self.HeroUI`) (/ (`self.Skill1_CD_real`) (`self.Skill1_CD`)))
  (`/Game/AllLogic/UI/HeroUse.SetSkill2 Progress` (`self.HeroUI`) (/ (`self.Skill2_CD_real`) (`self.Skill2_CD`)))
  (`/Game/AllLogic/UI/HeroUse.SetSkill3 Progress` (`self.HeroUI`) (/ (`self.Skill3_CD_real`) (`self.Skill3_CD`)))
  (`/Game/AllLogic/UI/HeroUse.SetSkill4 Progress` (`self.HeroUI`) (/ (`self.Skill4_CD_real`) (`self.Skill4_CD`))))

(event `Skill1`
  (if (>= (`self.Skill1_CD_real`) (`self.Skill1_CD`))
    (`/Game/AllLogic/UI/HeroUse.Skill1` (`self.HeroUI`))
    (set `self.Skill1_CD_real` 0.0)))

(event `self.ReceiveDrawHUD`
  (params (SizeX :type Integer) (SizeY :type Integer))
  (bind _returnvalue (`GameplayStatics.GetPlayerController` 0))
  (bind (_locationx _locationy) (`PlayerController.GetMousePosition` _returnvalue))
  (bind (_locationx_2 _locationy_2) (`PlayerController.GetMousePosition` _returnvalue))
  (`self.DrawText` (`KismetStringLibrary.Concat_StrStr` (`KismetStringLibrary.Concat_StrStr` (`KismetStringLibrary.Conv_DoubleToString` _locationx_2) ",") (`KismetStringLibrary.Conv_DoubleToString` _locationy_2)) (struct :`R` 1.0 :`G` 1.0 :`B` 1.0 :`A` 1.0) 256.0 0.0 "/Engine/EngineFonts/Roboto.Roboto")
  (`self.DrawMaterialSimple` "/Game/AllLogic/mouse/M_gam1541.M_gam1541" _locationx _locationy 50.0 50.0))

(event `Skill2`
  (if (>= (`self.Skill2_CD_real`) (`self.Skill2_CD`))
    (`/Game/AllLogic/UI/HeroUse.Skill2` (`self.HeroUI`))
    (set `self.Skill2_CD_real` 0.0)))

(event `Skill3`
  (if (>= (`self.Skill3_CD_real`) (`self.Skill3_CD`))
    (`/Game/AllLogic/UI/HeroUse.Skill3` (`self.HeroUI`))
    (set `self.Skill3_CD_real` 0.0)))

(event `Skill4`
  (if (>= (`self.Skill4_CD_real`) (`self.Skill4_CD`))
    (`/Game/AllLogic/UI/HeroUse.Skill4` (`self.HeroUI`))
    (set `self.Skill4_CD_real` 0.0)))

(fn `UserConstructionScript`)