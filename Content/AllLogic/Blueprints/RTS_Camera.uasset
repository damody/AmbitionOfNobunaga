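; RTS camera pawn or actor that takes over the player's view on BeginPlay, with screen-edge panning and mouse-wheel zoom.
; Each tick, a cursor within a few pixels of a viewport edge moves the root locally in that direction.
; Wheel input sets a clamped target boom length, which the spring arm eases toward with FInterpTo.
; ZoomCurve, sampled at the current arm length, scales both pan speed and zoom step.
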(event `self.ReceiveBeginPlay`
  (set `self.CamBoomLength` (`SpringArmComponent.TargetArmLength` (`self.SpringArm`)))
  (`PlayerController.SetViewTargetWithBlend` (`GameplayStatics.GetPlayerController` 0) self 0.0 "VTBlend_Linear" 0.0 false))

(event `self.ReceiveTick`
  (params (DeltaSeconds :type "Float (single-precision)"))
  (bind (_returnvalue_x _returnvalue_y) (`KismetMathLibrary.BreakVector2D` (`WidgetLayoutLibrary.GetViewportSize`)))
  (bind _springarm (`self.SpringArm`))
  (bind _returnvalue (* (`CurveFloat.GetFloatValue` (`self.ZoomCurve`) (`SpringArmComponent.TargetArmLength` (`self.SpringArm`))) 3.0))
  (bind _returnvalue_2 (* _returnvalue -1.0))
  (bind _asaon_player_controller (cast `/Game/AllLogic/Blueprints/AON_PlayerController` (`GameplayStatics.GetPlayerController` 0)))
  (`|ExecutionSequence`
    (:`then_0`
      (bind (_locationx _locationy) (`PlayerController.GetMousePosition` _asaon_player_controller))
      (bind (_x _y) (`KismetMathLibrary.BreakVector2D` (`KismetMathLibrary.MakeVector2D` _locationx _locationy)))
      (if (> _x (- _returnvalue_x 3.0))
        (`SceneComponent.K2_AddLocalOffset` (`self.DefaultSceneRoot`) (`KismetMathLibrary.MakeVector` 0.0 _returnvalue) false false)))
    (:`then_1`
      (if (< _x 3.0)
        (`SceneComponent.K2_AddLocalOffset` (`self.DefaultSceneRoot`) (`KismetMathLibrary.MakeVector` 0.0 _returnvalue_2) false false)))
    (:`then_2`
      (if (> _y (- _returnvalue_y 3.0))
        (`SceneComponent.K2_AddLocalOffset` (`self.DefaultSceneRoot`) (`KismetMathLibrary.MakeVector` _returnvalue_2) false false)))
    (:`then_3`
      (if (< _y 3.0)
        (`SceneComponent.K2_AddLocalOffset` (`self.DefaultSceneRoot`) (`KismetMathLibrary.MakeVector` _returnvalue) false false)))
    (:`then_4`
      (set `SpringArmComponent.TargetArmLength` (`KismetMathLibrary.FInterpTo` (`SpringArmComponent.TargetArmLength` _springarm) (`self.CamBoomLength`) DeltaSeconds 3.0) _springarm))))

(event `InputAction|Wheel Up`
  (params (Key :type "Key Structure" :default "AnyKey"))
  (bind _targetarmlength (`SpringArmComponent.TargetArmLength` (`self.SpringArm`)))
  (:`Pressed`
    (set `self.CamBoomLength` (`KismetMathLibrary.FClamp` (- _targetarmlength (* (`CurveFloat.GetFloatValue` (`self.ZoomCurve`) _targetarmlength) 50.0)) (`self.MinArm`) (`self.MaxArm`)))))

(event `InputAction|Wheel Down`
  (params (Key :type "Key Structure" :default "AnyKey"))
  (bind _targetarmlength (`SpringArmComponent.TargetArmLength` (`self.SpringArm`)))
  (:`Pressed`
    (set `self.CamBoomLength` (`KismetMathLibrary.FClamp` (+ (* (`CurveFloat.GetFloatValue` (`self.ZoomCurve`) _targetarmlength) 50.0) _targetarmlength) (`self.MinArm`) (`self.MaxArm`)))))

(fn `UserConstructionScript`)